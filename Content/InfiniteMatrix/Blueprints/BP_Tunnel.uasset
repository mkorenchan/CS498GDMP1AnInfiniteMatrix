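; BP_Tunnel is one tunnel segment with a rotating obstacle wall, a spinning health pack and an enemy.
; Randomize picks one of four hole meshes and a random roll, then shows and repositions each pickup or enemy by weighted chance.
; Overlaps report hits to BP_Player, while projectile kills on the enemy add score.
; Reaching TriggerZone makes TunnelSpawner spawn another tunnel, notifies the player and destroys this one.
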(event OnComponentBeginOverlap(TriggerZone)
  (params (OverlappedComponent :type Primitive%20Component%20Object%20Reference) (OtherActor :type Actor%20Object%20Reference) (OtherComp :type Primitive%20Component%20Object%20Reference) (OtherBodyIndex :type Integer) (bFromSweep :type Boolean) (SweepResult :type Hit%20Result%20Structure%20%28by%20ref%29))
  (bind _asbp_player (Utilities|Casting|CastToBP_Player OtherActor))
  (Default|SpawnTunnelatSpawnPoint (Variables|Default|GetTunnelSpawner))
  (Default|OverlapTunnelTrigger _asbp_player)
  (Actor|DestroyActor))

(event OnComponentBeginOverlap(WallMesh)
  (params (OverlappedComponent :type Primitive%20Component%20Object%20Reference) (OtherActor :type Actor%20Object%20Reference) (OtherComp :type Primitive%20Component%20Object%20Reference) (OtherBodyIndex :type Integer) (bFromSweep :type Boolean) (SweepResult :type Hit%20Result%20Structure%20%28by%20ref%29))
  (bind _asbp_player (Utilities|Casting|CastToBP_Player OtherActor))
  (Default|CollidewithObstacle _asbp_player))

(event OnComponentBeginOverlap(HealthPack)
  (params (OverlappedComponent :type Primitive%20Component%20Object%20Reference) (OtherActor :type Actor%20Object%20Reference) (OtherComp :type Primitive%20Component%20Object%20Reference) (OtherBodyIndex :type Integer) (bFromSweep :type Boolean) (SweepResult :type Hit%20Result%20Structure%20%28by%20ref%29))
  (bind _asbp_player (Utilities|Casting|CastToBP_Player OtherActor))
  (Default|CollidewithHealthPack _asbp_player)
  (Components|DestroyComponent (Variables|Default|GetHealthPack)))

(event OnComponentBeginOverlap(Enemy)
  (params (OverlappedComponent :type Primitive%20Component%20Object%20Reference) (OtherActor :type Actor%20Object%20Reference) (OtherComp :type Primitive%20Component%20Object%20Reference) (OtherBodyIndex :type Integer) (bFromSweep :type Boolean) (SweepResult :type Hit%20Result%20Structure%20%28by%20ref%29))
  (bind _enemy (Variables|Default|GetEnemy))
  (bind _asbp_player (Utilities|Casting|CastToBP_Player OtherActor)
    (:then
      (Default|CollidewithEnemy _asbp_player))
    (:CastFailed
      (Utilities|Casting|CastToBP_Projectile OtherActor)
      (bind _asbp_player_2 (Utilities|Casting|CastToBP_Player (Game|Player|GetPlayerPawn 0)))
      (Math|Integer|IncrementInt (Variables|/Game/InfiniteMatrix/Blueprints/BP_Player.BP_Player_C|GetScore _asbp_player_2)
        (:%20%20
          _))))
  (Effects|SpawnEmitteratLocation "/Game/StarterContent/Particles/P_Explosion.P_Explosion" (Transformation|GetWorldLocation _enemy) "0, 0, 0" "5.000000,5.000000,5.000000")
  (Components|DestroyComponent _enemy))

(event EventBeginPlay)

(event EventTick
  (params (DeltaSeconds :type Float%20%28single-precision%29))
  (bind _healthpack (Variables|Default|GetHealthPack))
  (Transformation|AddLocalRotation (Variables|Default|GetWallMesh) (Math|Rotator|MakeRotator (* DeltaSeconds (Variables|Default|GetWallRotateSpeed)) 0.0 0.0) false false)
  (Utilities|IsValid _healthpack
    (:Is%20Valid
      (Transformation|AddLocalRotation _healthpack (Math|Rotator|MakeRotator (* DeltaSeconds (Variables|Default|GetHealthPackRotateSpeed)) 0.0 0.0) false false))))

(fn ConstructionScript)

(fn Randomize
  (bind _returnvalue (Math|Random|RandomFloatinRange -2.5e+02 2.5e+02))
  (bind _returnvalue_2 (Math|Random|RandomFloatinRange -2.5e+02 2.5e+02))
  (bind _healthpack (Variables|Default|GetHealthPack))
  (bind _wallmesh (Variables|Default|GetWallMesh))
  (bind _enemy (Variables|Default|GetEnemy))
  ;[1 1 1] Spawn Obstacle
  (Components|StaticMesh|SetStaticMesh _wallmesh (Utilities|Select :Index (Math|Random|RandomIntegerinRange 0 3) :Option%200 "/Game/InfiniteMatrix/Meshes/SM_Hole_01.SM_Hole_01" :Option%201 "/Game/InfiniteMatrix/Meshes/SM_Hole_02.SM_Hole_02" :Option%202 "/Game/InfiniteMatrix/Meshes/SM_Hole_03.SM_Hole_03" :Option%203 "/Game/InfiniteMatrix/Meshes/SM_Hole_04.SM_Hole_04"))
  (Transformation|AddLocalRotation _wallmesh (Math|Rotator|MakeRotator (Math|Random|RandomFloatinRange 0.0 3.6e+02) 0.0 0.0) false false)
  ;[1 1 1] Randomize Health Pack
  (Utilities|IsValid _healthpack
    (:Is%20Valid
      (bind _output_get (LocalVariables|SetnewHidden (not (Math|Random|RandomBoolwithWeight (Variables|Default|GetHealthPackProbability)))))
      (Development|SetHiddeninGame _healthpack _output_get true)
      (Collision|SetCollisionEnabled _healthpack (select _output_get (Utilities|Enum|LiteralenumECollisionEnabled "NoCollision") "QueryOnly"))
      (Transformation|SetRelativeTransform _healthpack (Math|Transform|MakeTransform (Math|Vector|MakeVector (Math|Random|RandomFloatinRange 5e+02 2e+03) _returnvalue _returnvalue) "90.000000,0.000000,0.000000" "1,1,1") false false))
    (:Is%20Not%20Valid
      _))
  ;[1 1 1] Randomize Enemy
  (Utilities|IsValid _enemy
    (:Is%20Valid
      (bind _output_get_2 (LocalVariables|SetnewHidden (not (Math|Random|RandomBoolwithWeight (Variables|Default|GetEnemyProbability)))))
      (Development|SetHiddeninGame _enemy _output_get_2 true)
      (Collision|SetCollisionEnabled _enemy (select _output_get_2 (Utilities|Enum|LiteralenumECollisionEnabled "NoCollision") "QueryOnly"))
      (Transformation|SetRelativeTransform _enemy (Math|Transform|MakeTransform (Math|Vector|MakeVector (Math|Random|RandomFloatinRange 5e+02 2e+03) _returnvalue_2 _returnvalue_2) "0,90.000000, 0" "1,1,1") false false))))