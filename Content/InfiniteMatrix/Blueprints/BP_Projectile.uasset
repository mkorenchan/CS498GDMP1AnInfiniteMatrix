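; BP_Projectile is a projectile actor that travels along world X at a speed derived from the player's speed.
; Each Tick it measures its mesh's distance to the player pawn, destroying itself beyond MaxDistanceFromPlayer.
; Otherwise it makes a swept world-offset move scaled by delta time and BP_Player's CurrentSpeed and ProjectileSpeedModifier.
; Any overlap on the projectile mesh also destroys it, with no damage or hit logic here.
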(event OnComponentBeginOverlap(ProjectileMesh)
  (params (OverlappedComponent :type Primitive%20Component%20Object%20Reference) (OtherActor :type Actor%20Object%20Reference) (OtherComp :type Primitive%20Component%20Object%20Reference) (OtherBodyIndex :type Integer) (bFromSweep :type Boolean) (SweepResult :type Hit%20Result%20Structure%20%28by%20ref%29))
  (Actor|DestroyActor))

(event EventBeginPlay)

(event Collision|EventActorBeginOverlap
  (params (OtherActor :type Actor%20Object%20Reference)))

(event EventTick
  (params (DeltaSeconds :type Float%20%28single-precision%29))
  ;[1 1 1] Advance Projectile
  (Math|Float|CompareFloat (Math|Vector|Distance(Vector) (Transformation|GetWorldLocation (Variables|Default|GetProjectileMesh)) (Transformation|GetWorldLocation (Variables|/Script/Engine.Actor|GetRootComponent (Game|Player|GetPlayerPawn 0)))) (Variables|Default|GetMaxDistanceFromPlayer)
    (:>
      (Actor|DestroyActor))
    (:==
      (bind _asbp_player (Utilities|Casting|CastToBP_Player (Game|Player|GetPlayerPawn 0) :!label _label))
      (Transformation|AddActorWorldOffset (Math|Vector|MakeVector (* DeltaSeconds (Variables|/Game/InfiniteMatrix/Blueprints/BP_Player.BP_Player_C|GetCurrentSpeed _asbp_player) (Variables|/Game/InfiniteMatrix/Blueprints/BP_Player.BP_Player_C|GetProjectileSpeedModifier _asbp_player)) 0.0 0.0) true))
    (:<
      (goto _label))))

(fn ConstructionScript)